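; Player Blueprint for a roleplay mode, handling each player's job, money, salary and F4 menu.
; The server spawns the job as an owned actor from an enum-keyed struct array and pays its salary on a looping timer.
; RepNotifies refresh the local HUD, and job changes, including remote players', also update the local F4 menu.
; Menu requests pass through client-to-server events, though entity purchases so far only print an affordability check.
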(event Custom|ServerChangeJob
  (params (JobEnum :type JobEnum%20Enum :default "NewEnumerator0"))
  ;[1 1 1] Change Job event on the server
  (Class|KJModProxy|PrintStringKJMod 0 "Server side change job" true true "(R=0.092105,G=1.000000,B=0.000000,A=1.000000)" 5.0)
  (Jobs|SetJobServer JobEnum) ; Set Job to selected job
)

(event Custom|ClientChangeJob
  (params (JobEnum :type JobEnum%20Enum :default "NewEnumerator0"))
  ;[1 1 1] CLIENT CHANGE JOB - The RP Menu has told us that it want's to change job, ask server to
  (Class|KJModProxy|PrintStringKJMod 0 (Utilities|String|Append "Client change job to " (Utilities|String|EnumtoString JobEnum)) true true "(R=0.092105,G=1.000000,B=0.000000,A=1.000000)" 5.0)
  (CallFunction|ServerChangeJob JobEnum) ; Calls the server side event for changing job
)

(event Custom|ClientBuyingEntity
  (params (EntityEnum :type EntityEnum%20Enum :default "NewEnumerator0"))
  ;[1 1 1] CLIENT BUY ENTITY - The rp menu told us that it wants to buy a entity, ask the server to do it
  (CallFunction|ServerBuyingEntity EntityEnum))

(event Custom|ServerBuyingEntity
  (params (EntityEnum :type EntityEnum%20Enum :default "NewEnumerator0"))
  ;[1 1 1] SERVER BUY ENTITY - Client told us it wants to buy a entity
  (Entities|BuyEntityServer EntityEnum))

(event EventPlayerSpawnedwithPawn
  ;[1 1 1] Player Spawned with Pawn - Built in event that handles what should happen when the player spawns in the world.
  ;;[1 1 1] Check if client and local player.
  (Utilities|HandleClientServerLogic
    (:ClientLogic
      (Utilities|IsLocalorRemote
        (:IsLocalPlayer
          (Default|SetJob (Variables|UIWidgets|GetLocalPlayerHudWidgetBP) (Variables|Default|GetPlayerJob))
          (HUD|UpdateMoneyClient))))))

(event EventBeginPlay)

(event EventInitialised
  ;[1 1 1] Player Initalised - Built in event that handles what should happen when the player first joins the server.
  (Jobs|MakeJobsArray) ; Creates an array of all the available jobs.
  (Entities|MakePrintersArray) ; Creates an array of all available printers.
  ;;[1 1 1] Checks if client or server.
  (Utilities|HandleClientServerLogic
    (:ServerLogic
      (Jobs|SetJobServer "NewEnumerator0") ; Sets the default job for the player.
      (Money|SetMoneyServer 1000) ; Sets the current money (will in the future pull amount for database)
      (Utilities|Time|SetTimerbyFunctionName 0 "GiveSalaryServer" 5.0 true))
    (:ClientLogic
      (Utilities|IsLocalorRemote ; Checks if its the local player (hud should only run on the local player).
        (:IsLocalPlayer
          ;;[1 1 1] Creates custom hud, adds it to the viewport and sets the correct input mode (focus on game so we can move character).
          (bind _returnvalue (UserInterface|CreateWidget "/Game/CustomContent/UGC2248027258/Blueprints/UI/LocalPlayerHudWidgetBP.LocalPlayerHudWidgetBP_C" (Game|GetPlayerController 0)))
          (Variables|UIWidgets|SetLocalPlayerHudWidgetBP _returnvalue)
          (UserInterface|Viewport|AddtoViewport _returnvalue 0)
          (Class|KJModPlayerProxy|SetInputMode "GameFocused" _returnvalue)
          (bind _returnvalue_2 (UserInterface|CreateWidget "/Game/CustomContent/UGC2248027258/Blueprints/UI/F4Menu/LocalPlayerF4WidgetBP.LocalPlayerF4WidgetBP_C" (Game|GetPlayerController 0))) ; Create f4 menu widget
          (Variables|UIWidgets|SetLocalPlayerF4WidgetBP _returnvalue_2) ; Set the f4 widget variable to later add it to the viewport.
          (Variables|/Game/CustomContent/UGC2248027258/Blueprints/UI/F4Menu/LocalPlayerF4WidgetBP.LocalPlayerF4WidgetBP_C|SetPlayer _returnvalue_2 self)
          ;;[1 1 1] So we can receive keys (like C for equipment, E for bodyscan, etc.)
          (Input|EnableInput (Game|GetPlayerController 0)))))))

(event Custom|ClientToggleF4Menu
  (bind _localplayerf4widgetbp (Variables|UIWidgets|GetLocalPlayerF4WidgetBP))
  (bind _localplayerf4widgetbp_2 (Variables|UIWidgets|GetLocalPlayerF4WidgetBP))
  ;[1 1 1] Toggle F4 Menu
  (if (not (UserInterface|Viewport|IsinViewport (Variables|UIWidgets|GetLocalPlayerF4WidgetBP))) ; Check if menu is visible
    (UserInterface|Viewport|AddtoViewport _localplayerf4widgetbp_2 2) ; Add menu to be visible in the viewport
    (Class|KJModPlayerProxy|SetInputMode "UserInterfaceFocused" _localplayerf4widgetbp_2) ; Show mouse
    (Default|ShowAvailableJobs (Variables|/Game/CustomContent/UGC2248027258/Blueprints/UI/F4Menu/LocalPlayerF4WidgetBP.LocalPlayerF4WidgetBP_C|GetLocalPlayerJobsWidgetBP _localplayerf4widgetbp) (Variables|Default|GetJobss))
    (Default|ShowAvailableBuyableEntities (Variables|/Game/CustomContent/UGC2248027258/Blueprints/UI/F4Menu/LocalPlayerF4WidgetBP.LocalPlayerF4WidgetBP_C|GetLocalPlayerEntitiesWidgetBP _localplayerf4widgetbp) (Variables|Default|GetBuyableEntities))
    (else
      (Widget|RemovefromParent _localplayerf4widgetbp_2)
      (Class|KJModPlayerProxy|SetInputMode "GameFocused" _localplayerf4widgetbp_2) ; Hide mouse
    )))

(event Input|KeyboardEvents|F4
  (params (Key :type Key%20Structure))
  ;[1 1 1] F4 Button action binding
  (:Released
    (bind _returnvalue (Class|KJModPlayerProxy|GetLocalPlayerProxy))
    (bind _asvanilla_rpplayer_bp (Utilities|Casting|CastToVanillaRPPlayerBP _returnvalue))
    (CallFunction|ClientToggleF4Menu _asvanilla_rpplayer_bp) ; Call toggle f4 menu event
  ))

(fn ConstructionScript)

(fn OnRepPlayerJob
  (bind _localplayerhudwidgetbp (Variables|UIWidgets|GetLocalPlayerHudWidgetBP))
  ;[1 1 1] Check if client and local player.
  (Utilities|HandleClientServerLogic
    (:ClientLogic
      (Utilities|IsLocalorRemote
        (:IsLocalPlayer
          ;[1 1 1] Update the player HUD
          (if (Utilities|IsValid _localplayerhudwidgetbp)
            (Default|SetJob _localplayerhudwidgetbp (Variables|Default|GetPlayerJob))
            ;[1 1 1] SOmething changes, ask F4 menu (to ask jobs section) to update itself
            (if (UserInterface|Viewport|IsinViewport (Variables|UIWidgets|GetLocalPlayerF4WidgetBP))
              (Default|UpdateAvailableJobs (Variables|UIWidgets|GetLocalPlayerF4WidgetBP) (Variables|Default|GetJobss)))))
        (:IsRemotePlayer
          ;[1 1 1] A remote user has picked a job.. we need to tell our "local" UI to update itself
          (bind _returnvalue (Class|KJModPlayerProxy|GetLocalPlayerProxy)) ; Remote user picked a new job, find "us"..
          (bind _asvanilla_rpplayer_bp (Utilities|Casting|CastToVanillaRPPlayerBP _returnvalue)) ; Turn into us
          (Default|UpdateAvailableJobs (Variables|VanillaRPPlayerBP_C|GetLocalPlayerF4WidgetBP _asvanilla_rpplayer_bp) (Variables|VanillaRPPlayerBP_C|GetJobss _asvanilla_rpplayer_bp)))))))

(fn MakeJobsArray
  ;[1 1 1] Makes an array of all the available jobs.
  (Utilities|FlowControl|Sequence
    (:then_0
      (Utilities|Array|Add (Variables|Default|GetJobss) (Utilities|Struct|MakeJobStructBP "NewEnumerator0" "/Game/CustomContent/UGC2248027258/Blueprints/Jobs/CitizenBP.CitizenBP_C" "Citizen" "Citizens are the backbone of the community and economy. This is the default class which gives you a solid salary just for existing. Use this one to base and print that sweet sweet moola." 45 999)))
    (:then_1
      (Utilities|Array|Add (Variables|Default|GetJobss) (Utilities|Struct|MakeJobStructBP "NewEnumerator3" "/Game/CustomContent/UGC2248027258/Blueprints/Jobs/ThiefBP.ThiefBP_C" "Thief" "Thieves are sly fuckers that steal and lie their way through life. Use this job to take stuff from the rich... and keep them to yourself. Kinda like a shitty Robin Hood." 10 4)))))

(fn SetJobServer
  (params (JobEnum :type JobEnum%20Enum :default "NewEnumerator0"))
  ;[1 1 1] Set Job - Sets the players job on the server side.
  (Utilities|HandleClientServerLogic ; Nt required
    (:ServerLogic
      (if (Utilities|IsValid (Variables|Default|GetPlayerJob))
        (Actor|DestroyActor (Variables|Default|GetPlayerJob)))
      (bind _jobstruct (Jobs|GetJobStructfromJobEnum JobEnum)) ; Convert enum to struct
      (bind _returnvalue (Game|SpawnActorfromClass (Utilities|Struct|BreakJobStructBP _jobstruct) (Math|Transform|MakeTransform "0, 0, 0") "Undefined" self 0)) ; Spawn the job based on the struct with the correct class. \nIMPORTANT:\nMake sure to set the owner so that the job knows what player spawned it.
      (Default|ConstructJob _returnvalue _jobstruct) ; Trigger the Construct Job function on the job BP.
      (Variables|Default|SetPlayerJob _returnvalue) ; Sets the job variable on the player.
    )))

(fn GetJobStructfromJobEnum
  (params (JobEnum :type JobEnum%20Enum :default "NewEnumerator0"))
  ;[1 1 1] Converts a job enum into the correct job struct based on the jobs array.
  ;;[1 1 1] Loop through all the available jobs.
  (for _array_element (Variables|Default|GetJobss)
    ;;[1 1 1] If we find the correct job from the array we return that job struct.
    (if (Utilities|Enum|Equal(Enum) (.JobEnum (Utilities|Struct|BreakJobStructBP _array_element)) JobEnum)
      (return _array_element))))

(fn OnRepPlayerMoney
  ;[1 1 1] Replication Notify for Player Money - When the money on the player is updated we want to update the hud.
  (HUD|UpdateMoneyClient))

(fn AddMoneyServer
  (params (Money :type Integer))
  ;[1 1 1] Add Money - Increase the players money with a certain amount.
  (Money|SetMoneyServer (+ Money (Variables|Default|GetPlayerMoney))) ; Sets money to amount
)

(fn SetMoneyServer
  (params (Money :type Integer))
  ;[1 1 1] Set the money - Sets the money on the server and notifies through replication.
  (Variables|Default|SetPlayerMoney Money) ; If server we set the money and notify the clients.
)

(fn GiveSalaryServer
  ;[1 1 1] Give Salary - Add the salary to the players money count.
  (Class|KJModProxy|PrintStringKJMod 0 "GIving player salary" true true "(R=1.000000,G=0.049471,B=0.000000,A=1.000000)" 5.0)
  (Money|AddMoneyServer (Variables|/Game/CustomContent/UGC2248027258/Blueprints/Jobs/BaseJobBP.BaseJobBP_C|GetJobSalary (Variables|Default|GetPlayerJob))))

(fn UpdateMoneyClient
  (bind _localplayerhudwidgetbp (Variables|UIWidgets|GetLocalPlayerHudWidgetBP))
  ;[1 1 1] Check if client and local player.
  (Utilities|HandleClientServerLogic
    (:ClientLogic
      (Utilities|IsLocalorRemote
        (:IsLocalPlayer
          (if (Utilities|IsValid _localplayerhudwidgetbp)
            (Rendering|Components|TextRender|SetText (Variables|/Game/CustomContent/UGC2248027258/Blueprints/UI/LocalPlayerHudWidgetBP.LocalPlayerHudWidgetBP_C|GettxtPlayerMoney _localplayerhudwidgetbp) (Utilities|Text|ToText(String) (Utilities|String|Append "$" (Utilities|String|ToString(Integer) (Variables|Default|GetPlayerMoney))))) ; Set the text in the hud for the money amount.
          ))))))

(fn MakePrintersArray
  (Utilities|FlowControl|Sequence
    (:then_0
      (Utilities|Array|Add (Variables|Default|GetBuyableEntities) (Utilities|Struct|MakeEntityStruct "NewEnumerator0" "/Game/CustomContent/UGC2248027258/Blueprints/Entities/Printers/BasePrinterBP.BasePrinterBP_C" "/Game/CustomContent/UGC2248027258/Textures/VanillaRPWorkshopLogo.VanillaRPWorkshopLogo" "Gold Money Printer" "Prints money, but not that fast." 5000 "NewEnumerator0" "NewEnumerator0")))
    (:then_1
      (Utilities|Array|Add (Variables|Default|GetBuyableEntities) (Utilities|Struct|MakeEntityStruct "NewEnumerator1" "/Game/CustomContent/UGC2248027258/Blueprints/Entities/Printers/GoldPrinterBP.GoldPrinterBP_C" "/Game/CustomContent/UGC2248027258/Textures/VanillaRPWorkshopLogo.VanillaRPWorkshopLogo" "Emerald Money Printer" "Prints money, but not as fast as possible." 50000 "NewEnumerator0" "NewEnumerator0")))))

(fn BuyEntityServer
  (params (EntityEnum :type EntityEnum%20Enum :default "NewEnumerator0"))
  (Utilities|HandleClientServerLogic ; Nt required
    (:ServerLogic
      (bind _entitystruct (Entities|GetEntityStructfromEntityEnum EntityEnum))
      (bind _can (Money|CanAffordServer (.entityprice _entitystruct)))
      (if _can
        (Development|PrintString "PLayer can afford the entity")
        (else
          (Development|PrintString "PLayer cant afford the entity"))))))

(fn GetEntityStructfromEntityEnum
  (params (EntityEnum :type EntityEnum%20Enum :default "NewEnumerator0"))
  (for _array_element (Variables|Default|GetBuyableEntities)
    (if (Utilities|Enum|Equal(Enum) (.EntityEnum (Utilities|Struct|BreakEntityStruct _array_element)) EntityEnum)
      (return _array_element))))

(fn CanAffordServer
  (params (Cost :type Integer))
  (return (> (Variables|Default|GetPlayerMoney) Cost)))