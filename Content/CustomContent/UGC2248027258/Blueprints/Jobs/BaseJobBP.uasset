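; Base job Blueprint for a roleplay mod, spawned by the player to hold that player's job name, salary and job enum.
; ConstructJob fills these from a job struct, and their OnRep handlers are empty stubs.
; UpdateHud writes the job name to the owning player's HUD on the local client only, using a proxy-controller check to tell local from remote players, but nothing here calls it.
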(event EventBeginPlay
  ;[1 1 1] BeginPlay - The job has been spawned by the player and we want to do stuff.
  (Class|KJModProxy|PrintStringKJMod 0 "Job Begin play" false true "(R=0.000000,G=1.000000,B=0.000000,A=1.000000)" 5.0))

(event EventDestroyed
  (Class|KJModProxy|PrintStringKJMod 0 "Job Destroyed" true true "(R=0.000000,G=1.000000,B=0.000000,A=1.000000)" 5.0))

(fn ConstructionScript)

(fn ConstructJob
  (params (JobStruct :type Job%20Struct%20BP%20Structure))
  ;[1 1 1] Construct Job - Gets run from the player to set the job information.
  (Variables|Default|SetJobName (.jobname JobStruct)) ; Set job name and notify
  (Variables|Default|SetJobSalary (.jobsalary JobStruct)) ; Set job salary and notify
  (Variables|Default|SetJobEnum (.jobenum JobStruct)))

(fn OnRepJobSalary
  ;[1 1 1] Job Salary was updated - Future use
)

(fn OnRepJobName
  ;[1 1 1] Job Name Updated - The job name was updated so we want to update the hud to display the new job name for the player.
)

(fn UpdateHud
  ;[1 1 1] Update Job Name - Triggers a Hud update for the job name.
  ;;[1 1 1] Check if client and if local player
  (Utilities|HandleClientServerLogic
    (:ClientLogic
      (Utilities|IsLocalorRemote
        (:IsLocalPlayer
          (bind _asvanilla_rpplayer_bp (Utilities|Casting|CastToVanillaRPPlayerBP (Components|GetOwner))) ; Casts the owner to the custom player representation
          (if (Utilities|IsValid (Variables|/Game/CustomContent/UGC2248027258/Blueprints/Player/VanillaRPPlayerBP.VanillaRPPlayerBP_C|GetLocalPlayerHudWidgetBP _asvanilla_rpplayer_bp))
            (Rendering|Components|TextRender|SetText (Variables|/Game/CustomContent/UGC2248027258/Blueprints/UI/LocalPlayerHudWidgetBP.LocalPlayerHudWidgetBP_C|GettxtPlayerJob (Variables|/Game/CustomContent/UGC2248027258/Blueprints/Player/VanillaRPPlayerBP.VanillaRPPlayerBP_C|GetLocalPlayerHudWidgetBP _asvanilla_rpplayer_bp)) (Utilities|Text|ToText(String) (Variables|Default|GetJobName))) ; Grab name and set the text on the hud.
          ))))))

(fn OnRepJobEnum)