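; Server-side game mode proxy for the VanillaRP custom game mode, handling players as they join.
; On activation it applies default join parameters for incoming player proxies.
; Its PlayerHasJoined override spawns a VanillaRPPlayerBP owned by the joining controller and records it in the player list.
; It then initialises that proxy with pawn settings that disable noclip, spawns the player into the world and returns the proxy.
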(event EventGameModeActivated
  ;[1 1 1] Gamemode was activated on server
  (Class|KJModGameModeProxy|SetJoiningPlayersParameters (Utilities|Struct|MakeKJModGameModeProxyPlayerJoinParameters true 2.0)) ; Sets paramters for all joining proxies.
)

(fn ConstructionScript)

(fn PlayerHasJoined
  (params (joiningPlayerController :type Player%20Controller%20Object%20Reference))
  ;[1 1 1] Overrides SDK function "Player Has Joined"
  ;;[1 1 1] Spawn custom player representation and add it to the list of players
  (bind _returnvalue (Game|SpawnActorfromClass "/Game/CustomContent/UGC2248027258/Blueprints/Player/VanillaRPPlayerBP.VanillaRPPlayerBP_C" (Math|Transform|MakeTransform "0, 0, 0") "Undefined" joiningPlayerController 0))
  (Utilities|Array|Add (Variables|Default|GetPlayerRepresentation) _returnvalue)
  (Class|KJModPlayerProxy|Initialise _returnvalue joiningPlayerController self (Utilities|Struct|MakeKJModPlayerProxyPawnSettings 100 100 false false true)) ; Initialise player proxy with settings. This runs the initialise function on the player proxy
  (Class|KJModGameModeProxy|SpawnPlayer _returnvalue) ; Spawn the player into the world. This runs the spawn player function on the player proxy.
  (return _returnvalue))