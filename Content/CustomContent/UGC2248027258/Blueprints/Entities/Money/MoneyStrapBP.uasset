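; MoneyStrapBP is a spawnable money strap pickup that players collect with E.
; On use, the server branch adds its Money amount to the player, destroys the actor and sends the player a pickup message with the amount.
; It builds on BaseSpawnableEntityBP and supplies remote info text showing the amount and the collect prompt.
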(event EventPlayerUseEntity
  (params (Player :type Vanilla%20RP%20Player%20BP%20Object%20Reference))
  ;[1 1 1] Player Use Entity - Inherited from BaseSpawnableEntityBP
  (Utilities|HandleClientServerLogic
    (:ServerLogic
      (Default|AddMoneyServer Player (Variables|Default|GetMoney))
      (Actor|DestroyActor)
      (Default|ShowMessageServer Player (Utilities|String|Append "You have picked up $" (Utilities|String|ToString(Integer) (Variables|Default|GetMoney)) "!")) ; Shows a message on the client side for the player.
    )))

(fn ConstructionScript
  (|CallParentFunction))

(fn GetRemoteInfo
  (return (Utilities|String|Append "<b>Money Strap of $" (Utilities|String|ToString(Integer) (Variables|Default|GetMoney)) "</> 
" "Press E to collect the money!")))