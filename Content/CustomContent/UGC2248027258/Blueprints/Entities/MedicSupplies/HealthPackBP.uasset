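; HealthPackBP is a spawnable health pickup entity derived from BaseSpawnableEntityBP that players use to regain 100 HP.
; On use, the server branch adds health to the player, destroys the pack and sends that player a confirmation message.
; GetRemoteInfo supplies the prompt text telling players to press E.
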(event EventBeginPlay
  (|CallParentFunction) ; This node is disabled and will not be called.\nDrag off pins to build functionality.
)

(event Collision|EventActorBeginOverlap
  (params (OtherActor :type Actor%20Object%20Reference))
  (|CallParentFunction OtherActor) ; This node is disabled and will not be called.\nDrag off pins to build functionality.
)

(event EventTick
  (params (DeltaSeconds :type Float%20%28single-precision%29))
  (|CallParentFunction DeltaSeconds) ; This node is disabled and will not be called.\nDrag off pins to build functionality.
)

(event EventPlayerUseEntity
  (params (Player :type Vanilla%20RP%20Player%20BP%20Object%20Reference))
  ;[1 1 1] Player Use Entity - Inherited from BaseSpawnableEntityBP
  (Utilities|HandleClientServerLogic
    (:ServerLogic
      (Class|KJModPlayerProxy|AddHealth Player 1e+02) ; Add health to the player
      (Actor|DestroyActor)
      (Default|ShowMessageRemote Player "You have recieved 100HP!") ; Shows a message on the client side for the palyer who picked up the ammo.
    )))

(fn ConstructionScript
  (|CallParentFunction))

(fn GetRemoteInfo
  (return "<b>Health Pack</> 
Press E to gain 100HP!"))