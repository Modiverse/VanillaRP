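; Health pack crate entity for medic supplies that dispenses one health pack per player use until it is empty.
; Use spawns a HealthPackBP just above the crate's bounds on the server, decrements CurrentAmount and destroys the crate at zero.
; Server-side damage handling counts hits and destroys the crate on the fourth, although the author's note says third.
; GetRemoteInfo builds the prompt text showing remaining and maximum packs.
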(event EventBeginPlay
  (|CallParentFunction) ; This node is disabled and will not be called.\nDrag off pins to build functionality.
)

(event Collision|EventActorBeginOverlap
  (params (OtherActor :type Actor%20Object%20Reference))
  (|CallParentFunction OtherActor) ; This node is disabled and will not be called.\nDrag off pins to build functionality.
)

(event EventTick
  (params (DeltaSeconds :type Float%20%28single-precision%29))
  (|CallParentFunction DeltaSeconds) ; This node is disabled and will not be called.\nDrag off pins to build functionality.
)

(event Game|Damage|EventAnyDamage
  (params (Damage :type Float%20%28single-precision%29) (DamageType :type Damage%20Type%20Object%20Reference) (InstigatedBy :type Controller%20Object%20Reference) (DamageCauser :type Actor%20Object%20Reference))
  (bind _hitcounter (Variables|Default|GetHitCounter))
  ;[1 1 1] AnyDamage - Destory actor on 3rd hit
  (Utilities|HandleClientServerLogic
    (:ServerLogic
      (Math|Integer|IncrementInt _hitcounter
        (:%20%20
          (if (> _hitcounter 3)
            (Actor|DestroyActor)))))))

(event EventPlayerUseEntity
  (params (Player :type Vanilla%20RP%20Player%20BP%20Object%20Reference))
  (bind _self self)
  (bind _currentamount (Variables|Default|GetCurrentAmount))
  (bind _returnvalue (Transformation|GetActorLocation _self))
  ;[1 1 1] Player Use Entity - Inherited from BaseSpawnableEntityBP
  (Utilities|HandleClientServerLogic
    (:ServerLogic
      (Game|SpawnActorfromClass "/Game/CustomContent/UGC2248027258/Blueprints/Entities/MedicSupplies/HealthPackBP.HealthPackBP_C" (Math|Transform|MakeTransform (Math|Vector|MakeVector (.x _returnvalue) (.y _returnvalue) (+ (.z _returnvalue) (.z (.BoxExtent (Collision|GetActorBounds _self false false))) 15.0)) "0, 0, 0" "1,1,1") "Undefined" 0 0) ; Spawn a health pack from the crate
      (Math|Integer|DecrementInt _currentamount
        (:%20%20
          (if (<= _currentamount 0)
            (Actor|DestroyActor) ; Remove actor if crate is empty
          ))))))

(fn ConstructionScript
  (|CallParentFunction))

(fn GetRemoteInfo
  (return (Utilities|String|Append "<b>Health Pack Crate</> 
" (Utilities|String|Append "Holds: " (Utilities|String|ToString(Integer) (Variables|Default|GetCurrentAmount)) "/" (Utilities|String|ToString(Integer) (Variables|Default|GetMaxAmount)) " 
Press E to take one pack from crate."))))

(fn OnRepCurrentAmount)

(fn OnRepMaxAmount)