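; SMG ammo box pickup entity, built on the spawnable entity base, that gives a player 120 SMG rounds when used.
; On use, server logic adds the ammo, refreshes the player's current ammo, destroys the box and sends that player a pickup message.
; Any damage also destroys the box on the server, and GetRemoteInfo supplies the prompt to press E to collect it.
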(event EventBeginPlay
  (|CallParentFunction) ; This node is disabled and will not be called.\nDrag off pins to build functionality.
)

(event Collision|EventActorBeginOverlap
  (params (OtherActor :type Actor%20Object%20Reference))
  (|CallParentFunction OtherActor) ; This node is disabled and will not be called.\nDrag off pins to build functionality.
)

(event EventTick
  (params (DeltaSeconds :type Float%20%28single-precision%29))
  (|CallParentFunction DeltaSeconds) ; This node is disabled and will not be called.\nDrag off pins to build functionality.
)

(event Game|Damage|EventAnyDamage
  (params (Damage :type Float%20%28single-precision%29) (DamageType :type Damage%20Type%20Object%20Reference) (InstigatedBy :type Controller%20Object%20Reference) (DamageCauser :type Actor%20Object%20Reference))
  ;[1 1 1] AnyDamage - Destory actor on any damage
  (Utilities|HandleClientServerLogic
    (:ServerLogic
      (Actor|DestroyActor))))

(event EventPlayerUseEntity
  (params (Player :type Vanilla%20RP%20Player%20BP%20Object%20Reference))
  ;[1 1 1] Player Use Entity - Inherited from BaseSpawnableEntityBP
  (Utilities|HandleClientServerLogic
    (:ServerLogic
      (Variables|/Game/CustomContent/UGC2248027258/Blueprints/Player/VanillaRPPlayerBP.VanillaRPPlayerBP_C|SetAmmoSMGServer Player (+ (Variables|/Game/CustomContent/UGC2248027258/Blueprints/Player/VanillaRPPlayerBP.VanillaRPPlayerBP_C|GetAmmoSMGServer Player) 120))
      (Default|UpdateCurrentAmmoServer Player)
      (Actor|DestroyActor)
      (Default|ShowMessageServer Player "You have recieved 120 SMG ammo.") ; Shows a message on the client side for the palyer who picked up the ammo.
    )))

(fn ConstructionScript
  (|CallParentFunction))

(fn GetRemoteInfo
  (return "<b>SMG Ammo Box</> 
Press E to collect 120 smg bullets!"))