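; Base money printer entity that accumulates cash over time for players to collect on use.
; On the server, a looping timer grows the stored amount, and using the printer pays it to the player and resets it.
; A second timer destroys it after BaseExplodeTimer (the random offset integer-divides to zero), as does damage depleting its health.
; GetRemoteInfo builds the owner, balance and use-prompt text.
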(event Custom|PlayerEmptiesPrinter
  (params (Player :type Vanilla%20RP%20Player%20BP%20Object%20Reference))
  ;[1 1 1] Player Empties Printer SERVER - Handles player taking money from printer.
  (Default|AddMoneyServer Player (Variables|Default|GetCurrentAmount)) ; Add money to player
  (Variables|Default|SetCurrentAmount 0) ; Empty printer
)

(event EventBeginPlay
  (Utilities|HandleClientServerLogic
    (:ServerLogic
      (Utilities|Time|SetTimerbyFunctionName 0 "PrintMoneyServer" (Math|Conversions|ToFloat(Integer) (Variables|Default|GetPrintInterval)) true) ; Loop timer to add amount at certain interval
      (Utilities|Time|SetTimerbyFunctionName 0 "DestroyPrinterServer" (Math|Conversions|ToFloat(Integer) (+ (/ (Math|Random|RandomInteger 5) 10) (Variables|Default|GetBaseExplodeTimer)))))))

(event Game|Damage|EventAnyDamage
  (params (Damage :type Float%20%28single-precision%29) (DamageType :type Damage%20Type%20Object%20Reference) (InstigatedBy :type Controller%20Object%20Reference) (DamageCauser :type Actor%20Object%20Reference))
  ;[1 1 1] AnyDamage - Destory actor on any damage
  (Utilities|HandleClientServerLogic
    (:ServerLogic
      (Variables|Default|SetHealth (- (Variables|Default|GetHealth) (Math|Float|Truncate Damage)))
      (if (<= (Variables|Default|GetHealth) 0)
        (Actor|DestroyActor)))))

(event EventPlayerUseEntity
  (params (Player :type Vanilla%20RP%20Player%20BP%20Object%20Reference))
  (Utilities|HandleClientServerLogic
    (:ServerLogic
      (CallFunction|PlayerEmptiesPrinter Player))))

(fn ConstructionScript)

(fn PrintMoneyServer
  (Utilities|HandleClientServerLogic
    (:ServerLogic
      (Variables|Default|SetCurrentAmount (+ (Variables|Default|GetCurrentAmount) (Variables|Default|GetPrintAmount)))
      (Development|PrintString "Printed money"))))

(fn OnRepCurrentAmount)

(fn GetRemoteInfo
  (return (Utilities|String|Append (Utilities|String|Append (Utilities|String|Append (Utilities|String|Append "<b>" (Variables|Default|GetOwnerName)) "'s printer</> 
") (Utilities|String|Append "Holds: $" (Utilities|String|ToString(Integer) (Variables|Default|GetCurrentAmount)))) " 
Press E to take money.")))

(fn PlayerUseServer)

(fn DestroyPrinterServer
  (Actor|DestroyActor))