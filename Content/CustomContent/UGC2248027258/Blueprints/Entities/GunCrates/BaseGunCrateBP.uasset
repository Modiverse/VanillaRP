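; Base gun crate entity that hands out one gun each time a player uses it.
; On use it gives the configured item, shows and prints a pickup message, decrements the remaining count, and destroys itself when empty.
; Its remote info text shows the gun name, current and maximum count, and a use prompt.
; The name and count variables are RepNotify, with empty handlers.
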(event EventBeginPlay
  (|CallParentFunction) ; This node is disabled and will not be called.\nDrag off pins to build functionality.
)

(event Collision|EventActorBeginOverlap
  (params (OtherActor :type Actor%20Object%20Reference))
  (|CallParentFunction OtherActor) ; This node is disabled and will not be called.\nDrag off pins to build functionality.
)

(event EventTick
  (params (DeltaSeconds :type Float%20%28single-precision%29))
  (|CallParentFunction DeltaSeconds) ; This node is disabled and will not be called.\nDrag off pins to build functionality.
)

(event EventPlayerUseEntity
  (params (Player :type Vanilla%20RP%20Player%20BP%20Object%20Reference))
  (bind _gunname (Variables|Default|GetGunName))
  (bind _currentamount (Variables|Default|GetCurrentAmount))
  (bind _returnvalue (Utilities|String|Append "You just picked up a " _gunname "!"))
  (Class|KJModPlayerProxy|Give Player (Variables|Default|GetGunItemName))
  (Class|KJModPlayerProxy|ShowMessage Player _returnvalue 5 true)
  (Development|PrintString _returnvalue)
  (Math|Integer|DecrementInt _currentamount
    (:%20%20
      (if (<= _currentamount 0)
        (Actor|DestroyActor)))))

(fn ConstructionScript
  (|CallParentFunction))

(fn GetRemoteInfo
  (return (Utilities|String|Append (Utilities|String|Append "<b>" (Variables|Default|GetGunName) " Crate</> 
") (Utilities|String|Append "Holds: " (Utilities|String|ToString(Integer) (Variables|Default|GetCurrentAmount)) "/" (Utilities|String|ToString(Integer) (Variables|Default|GetMaxAmount)) " 
Press E to take one gun from crate."))))

(fn OnRepGunName)

(fn OnRepCurrentAmount)

(fn OnRepMaxAmount)